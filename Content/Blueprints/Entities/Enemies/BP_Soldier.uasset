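; BP_Soldier is an enemy Blueprint whose own graph drives the status effect display shown through its Widget component.
; On BeginPlay it casts and caches the WBP_StatusEffects widget, then injects its StatusEffectComponent into it.
; A UI update event refreshes the visuals.
; The widget is hidden on death and shown again when the enemy is taken from the pool, so it supports pooled reuse.
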(event `self.ReceiveBeginPlay`
  (bind _aswbp_status_effects (cast `/Game/Blueprints/Widgets/WBP_StatusEffects` (`WidgetComponent.GetWidget` (`self.Widget`))))
  (bind _output_get (set `self.StatusEffectVisuals` _aswbp_status_effects))
  (`/Game/Blueprints/Widgets/WBP_StatusEffects.InjectStatusEffect` _output_get (`self.StatusEffectComponent`)))

(event `self.OnUpdateStatusEffectUI`
  (`/Game/Blueprints/Widgets/WBP_StatusEffects.SetVisuals` (`self.StatusEffectVisuals`)))

(event `self.OnEnemyDeath`
  (`Widget.SetVisibility` (`self.StatusEffectVisuals`) "Hidden"))

(event `self.OnEnemyGotFromPool`
  (`Widget.SetVisibility` (`self.StatusEffectVisuals`) "Visible"))

(fn `UserConstructionScript`)