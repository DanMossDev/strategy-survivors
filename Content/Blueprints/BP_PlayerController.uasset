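; Player controller Blueprint that serves as the relay for pause and menu input in what appears to be a Toon Tanks game.
; On BeginPlay it adds the ToonTanksUI Enhanced Input mapping context.
; Pause, confirm, back and tab left/right actions each call a matching event dispatcher, leaving the response to listeners.
; A change to controller input likewise calls a setup-for-controller dispatcher.
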(event `self.OnInputChangedToController`
  (`self.OnSetupForController`))

(event `self.ReceiveBeginPlay`
  (`EnhancedInputSubsystemInterface.AddMappingContext` (pcsubsystem `EnhancedInputLocalPlayerSubsystem` self) "/Game/Input/ToonTanksUI.ToonTanksUI" 0 (struct)))

(event `EnhancedInput|/Game/Input/Pause`
  (params (ActionValue :type Boolean) (ElapsedSeconds :type "Float (double-precision)") (TriggeredSeconds :type "Float (double-precision)") (InputAction :type "InputAction Object Reference" :default "/Game/Input/Pause.Pause"))
  (:`Triggered`
    (`self.OnPausePressed`)))

(event `EnhancedInput|/Game/Input/UI/UI_Confirm`
  (params (ActionValue :type Boolean) (ElapsedSeconds :type "Float (double-precision)") (TriggeredSeconds :type "Float (double-precision)") (InputAction :type "InputAction Object Reference" :default "/Game/Input/UI/UI_Confirm.UI_Confirm"))
  (:`Triggered`
    (`self.OnSelect`)))

(event `EnhancedInput|/Game/Input/UI/UI_Back`
  (params (ActionValue :type Boolean) (ElapsedSeconds :type "Float (double-precision)") (TriggeredSeconds :type "Float (double-precision)") (InputAction :type "InputAction Object Reference" :default "/Game/Input/UI/UI_Back.UI_Back"))
  (:`Triggered`
    (`self.OnBack`)))

(event `EnhancedInput|/Game/Input/UI/UI_TabLeft`
  (params (ActionValue :type Boolean) (ElapsedSeconds :type "Float (double-precision)") (TriggeredSeconds :type "Float (double-precision)") (InputAction :type "InputAction Object Reference" :default "/Game/Input/UI/UI_TabLeft.UI_TabLeft"))
  (:`Triggered`
    (`self.OnTabLeft`)))

(event `EnhancedInput|/Game/Input/UI/UI_TabRight`
  (params (ActionValue :type Boolean) (ElapsedSeconds :type "Float (double-precision)") (TriggeredSeconds :type "Float (double-precision)") (InputAction :type "InputAction Object Reference" :default "/Game/Input/UI/UI_TabRight.UI_TabRight"))
  (:`Triggered`
    (`self.OnTabRight`)))

(fn `UserConstructionScript`)