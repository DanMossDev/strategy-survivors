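; BP_Puddle is an elemental puddle actor that shows visuals matching its Element.
; RefreshVisuals turns off all visuals, enables the set for the current Element, then prints a debug string.
; Shared helpers toggle each visual component's activation and in-game visibility, including its children.
; Only the Fire element has visuals wired up.
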(event `self.RefreshVisuals`
  (`self.DisableAllVisuals`)
  (`self.EnableSpecificVisuals` (`self.Element`))
  (`KismetSystemLibrary.PrintString` "Hello"))

(fn `DisableAllVisuals`
  (`self.DisableVisuals` (`self.FireVisuals`)))

(fn `DisableVisuals`
  (params (Visuals :type "SceneComponent Object Reference"))
  (`ActorComponent.Deactivate` Visuals)
  (`SceneComponent.SetHiddenInGame` Visuals true true))

(fn `EnableSpecificVisuals`
  (params (Element :type "EElementalType Enum" :default "None"))
  (switch `EElementalType` Element
    (:`Fire`
      (`self.EnableVisuals` (`self.FireVisuals`)))))

(fn `EnableVisuals`
  (params (Visuals :type "SceneComponent Object Reference"))
  (`ActorComponent.Activate` Visuals false)
  (`SceneComponent.SetHiddenInGame` Visuals false true))

(fn `UserConstructionScript`)