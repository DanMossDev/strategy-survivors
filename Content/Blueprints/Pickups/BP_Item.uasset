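; BP_Item is a pickup that, when picked up, offers the player an evolution or an item selection.
; OnPickedUp asks BP_ToonTanksGameMode for random evolveables and opens WBP_EvolutionScreen if any exist.
; Otherwise it queries uncached random unlockables and, if any exist, has the game mode set up item selection; with neither, nothing happens.
; The game mode reference is cast and stored in the construction script.
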(event `self.OnPickedUp`
  (bind _bpgamemode (`self.BPGameMode`))
  (bind _returnvalue (`ToonTanksGameMode.GetRandomEvolveable` _bpgamemode))
  (switch `int` (`KismetArrayLibrary.Array_Length` _returnvalue)
    (:`Default`
      (bind _returnvalue_2 (`|CreateWidget` "/Game/Blueprints/Widgets/WBP_EvolutionScreen.WBP_EvolutionScreen_C"))
      (`UserWidget.AddToViewport` _returnvalue_2 0)
      (`/Game/Blueprints/Widgets/WBP_EvolutionScreen.Setup` _returnvalue_2))
    (:`0`
      (bind _returnvalue_3 (`ToonTanksGameMode.GetRandomUnlockablesUncached` _bpgamemode))
      (switch `int` (`KismetArrayLibrary.Array_Length` _returnvalue_3)
        (:`Default`
          (`/Game/BP_ToonTanksGameMode.OnSetupItemSelect` (`self.BPGameMode`) false))))))

(fn `UserConstructionScript`
  (bind _asbp_toon_tanks_game_mode (cast `/Game/BP_ToonTanksGameMode` (`GameplayStatics.GetGameMode`)))
  (set `self.BPGameMode` _asbp_toon_tanks_game_mode))