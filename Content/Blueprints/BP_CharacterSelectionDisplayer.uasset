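; BP_CharacterSelectionDisplayer holds the display meshes for the selectable tank characters, judging by its name and components.
; On BeginPlay it registers each tank character data asset with its themed mesh component, such as ToyTank, GhostChef or Duck, through AddToCharacterMeshLookup.
; The graph only fills this lookup and contains no logic for switching or showing meshes, and the construction script is empty.
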(event `self.ReceiveBeginPlay`
  (`self.AddToCharacterMeshLookup` "/Game/Data/Characters/DA_StandardTank.DA_StandardTank" (`self.ToyTank`))
  (`self.AddToCharacterMeshLookup` "/Game/Data/Characters/DA_BoomerangTank.DA_BoomerangTank" (`self.GhostChef`))
  (`self.AddToCharacterMeshLookup` "/Game/Data/Characters/DA_FireTank.DA_FireTank" (`self.FireEngine`))
  (`self.AddToCharacterMeshLookup` "/Game/Data/Characters/DA_GatlingTank.DA_GatlingTank" (`self.Rat`))
  (`self.AddToCharacterMeshLookup` "/Game/Data/Characters/DA_IceTank.DA_IceTank" (`self.IceCreamVan`))
  (`self.AddToCharacterMeshLookup` "/Game/Data/Characters/DA_OilTank.DA_OilTank" (`self.Squid`))
  (`self.AddToCharacterMeshLookup` "/Game/Data/Characters/DA_WaterTank.DA_WaterTank" (`self.Duck`)))

(fn `UserConstructionScript`)