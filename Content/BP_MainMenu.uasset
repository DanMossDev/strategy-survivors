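; BP_MainMenu runs the main menu, applying a frame cap and saved sound volumes, then managing screens as a stack of widget classes.
; Main-to-character-select or milestones transitions play a level sequence before creating the widget, while options opens immediately.
; Pause or Back pops the stack, plays the return sequence and recreates the previous screen, quitting when empty.
; Global time dilation is near zero, hence the tiny transition delays.
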(event `self.ReceiveBeginPlay`
  (bind _returnvalue (`GameUserSettings.GetGameUserSettings`))
  (`GameUserSettings.SetFrameRateLimit` _returnvalue 144.0)
  (`GameUserSettings.ApplySettings` _returnvalue false)
  (bind _asbp_survivor_game_instance (cast `/Game/BP_SurvivorGameInstance` (`GameplayStatics.GetGameInstance`)))
  (bind _returnvalue_2 (`SurvivorGameInstance.GetSaveFile` _asbp_survivor_game_instance))
  (`GameplayStatics.SetSoundMixClassOverride` "/Game/Assets/Audio/Mix.Mix" "/Engine/EngineSounds/Master.Master" (`SaveFile.Volume` _returnvalue_2))
  (`GameplayStatics.SetSoundMixClassOverride` "/Game/Assets/Audio/Mix.Mix" "/Engine/EngineSounds/SFX.SFX" (`SaveFile.SFXVolume` _returnvalue_2))
  (`GameplayStatics.SetSoundMixClassOverride` "/Game/Assets/Audio/Mix.Mix" "/Engine/EngineSounds/Music.Music" (`SaveFile.MusicVolume` _returnvalue_2))
  (`self.ShowMainMenu`)
  (bind _asbp_player_controller (cast `/Game/Blueprints/BP_PlayerController` (`GameplayStatics.GetPlayerController` 0)))
  (add `/Game/Blueprints/BP_PlayerController.OnPausePressed` _asbp_player_controller (delegate `PausePressed`))
  (add `/Game/Blueprints/BP_PlayerController.OnBack` _asbp_player_controller (delegate `OnBack`))
  (`GameplayStatics.SetGlobalTimeDilation` 0.0001))

(event `PausePressed`
  (`self.RemoveFromStack` :!label _label))

(event `OnBack`
  (goto _label))

(event `AddToStackAfterSequence_Event`
  (params (Widget :type "UserWidget Class Reference") (Sequence :type "LevelSequenceActor Object Reference"))
  (`MovieSceneSequencePlayer.Play` (`LevelSequenceActor.SequencePlayer` Sequence))
  (`KismetSystemLibrary.Delay` 0.00015)
  (bind _returnvalue (`|CreateWidget` Widget))
  (`UserWidget.AddToViewport` _returnvalue 0)
  (`KismetArrayLibrary.Array_Add` (`self.UIScreenStack`) (`GameplayStatics.GetObjectClass` _returnvalue))
  (set `self.CurrentWidget` _returnvalue))

(event `RemoveFromStackAfterSequence_Event`
  (params (Widget :type "UserWidget Class Reference") (Sequence :type "LevelSequenceActor Object Reference"))
  (`MovieSceneSequencePlayer.Play` (`LevelSequenceActor.SequencePlayer` Sequence))
  (`KismetSystemLibrary.Delay` 0.00015)
  (bind _returnvalue (`|CreateWidget` Widget))
  (`UserWidget.AddToViewport` _returnvalue 0)
  (set `self.CurrentWidget` _returnvalue))

(fn `AddToStack`
  (params (ClassToAdd :type "UserWidget Class Reference"))
  (bind _currentwidget (`self.CurrentWidget`))
  (bind _maintocharacterselectsequence (`self.MainToCharacterSelectSequence`))
  (if (`KismetSystemLibrary.IsValid` _currentwidget)
    (`Widget.RemoveFromParent` _currentwidget)
    (if (== ClassToAdd "/Game/Blueprints/Widgets/MainMenu/WBP_OptionsMenu.WBP_OptionsMenu_C")
      (bind _returnvalue (`|CreateWidget` ClassToAdd :!label _label))
      (`UserWidget.AddToViewport` _returnvalue 0)
      (`KismetArrayLibrary.Array_Add` (`self.UIScreenStack`) (`GameplayStatics.GetObjectClass` _returnvalue))
      (set `self.CurrentWidget` _returnvalue)
      (elif (== (`GameplayStatics.GetObjectClass` _currentwidget) "/Game/Blueprints/Widgets/MainMenu/WBP_MainMenu.WBP_MainMenu_C")
        (if (== ClassToAdd "/Game/Blueprints/Widgets/MainMenu/WBP_CharacterSelect.WBP_CharacterSelect_C")
          (`self.AddToStackAfterSequence_Event` ClassToAdd _maintocharacterselectsequence)
          (elif (== ClassToAdd "/Game/Blueprints/Widgets/MainMenu/WBP_MilestonesScreen.WBP_MilestonesScreen_C")
            (`self.AddToStackAfterSequence_Event` ClassToAdd _maintocharacterselectsequence)))))
    (else
      (goto _label))))

(fn `RemoveFromStack`
  (bind _uiscreenstack (`self.UIScreenStack`))
  (bind _characterselecttomainsequence (`self.CharacterSelectToMainSequence`))
  (bind _returnvalue (- (`KismetArrayLibrary.Array_Length` _uiscreenstack) 1))
  (if (> (`KismetArrayLibrary.Array_Length` _uiscreenstack) 0)
    (`Widget.RemoveFromParent` (`self.CurrentWidget`))
    (`KismetArrayLibrary.Array_Remove` _uiscreenstack _returnvalue)
    (if (> (`KismetArrayLibrary.Array_Length` _uiscreenstack) 0)
      (bind _aslevel_sequence_actor (cast `LevelSequenceActor` (`KismetMathLibrary.SelectObject` _characterselecttomainsequence _characterselecttomainsequence (== (`GameplayStatics.GetObjectClass` (`self.CurrentWidget`)) "/Game/Blueprints/Widgets/MainMenu/WBP_CharacterSelect.WBP_CharacterSelect_C"))))
      (`self.RemoveFromStackAfterSequence_Event` (`|GetArrayItem` _uiscreenstack _returnvalue) _aslevel_sequence_actor)
      (else
        (`KismetSystemLibrary.QuitGame` null "Quit")))))

(fn `ShowMainMenu`
  (`WidgetLayoutLibrary.RemoveAllWidgets`)
  (`self.AddToStack` "/Game/Blueprints/Widgets/MainMenu/WBP_MainMenu.WBP_MainMenu_C"))

(fn `UserConstructionScript`)